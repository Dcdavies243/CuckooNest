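; Barwell is an AI pawn Blueprint that tracks which of two patrol points is its current destination.
; On BeginPlay it writes CurrentPatrolPoint to its blackboard as an object value, though the key name is left as None.
; Overlapping either patrol point switches CurrentPatrolPoint to the other one, without writing the change back to the blackboard.
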(event EventBeginPlay
  ;[1 1 1] When character spawned, set blackboard key to Patrol Point
  (AI|Components|Blackboard|SetValueasObject (AI|GetBlackboard self) (Utilities|Name|MakeLiteralName "None") (Variables|Default|GetCurrentPatrolPoint)))

(event Collision|EventActorBeginOverlap
  (params (OtherActor :type Actor%20Object%20Reference))
  (if (== OtherActor (Variables|Default|GetPatrolPoint1))
    (Variables|Default|SetCurrentPatrolPoint (Variables|Default|GetPatrolPoint2))
    (elif (== OtherActor (Variables|Default|GetPatrolPoint2))
      (Variables|Default|SetCurrentPatrolPoint (Variables|Default|GetPatrolPoint1)))))

(fn ConstructionScript)